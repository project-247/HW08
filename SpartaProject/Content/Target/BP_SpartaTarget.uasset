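; BP_SpartaTarget is a pop-up shooting target that stands up, gets knocked down and awards score.
; A state machine moves from Ready through Standing to KnockedDown: trigger volumes entered by BP_SpartaCharacter stand it up, knock it down or reset it.
; BP_Bullet hits on the board also knock it down.
; Tick applies timed incremental pitch rotation, completing each transition state when the timer expires.
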(event OnActorBeginOverlap(StandUpVolume)
  (params (OverlappedActor :type Actor%20Object%20Reference) (OtherActor :type Actor%20Object%20Reference))
  (Utilities|Casting|CastToBP_SpartaCharacter OtherActor)
  (CallFunction|StandUp))

(event OnActorBeginOverlap(KnockDownVolume)
  (params (OverlappedActor :type Actor%20Object%20Reference) (OtherActor :type Actor%20Object%20Reference))
  (Utilities|Casting|CastToBP_SpartaCharacter OtherActor)
  (CallFunction|KnockDown))

(event OnActorBeginOverlap(ResetVolume)
  (params (OverlappedActor :type Actor%20Object%20Reference) (OtherActor :type Actor%20Object%20Reference))
  (Utilities|Casting|CastToBP_SpartaCharacter OtherActor)
  (if (Utilities|Enum|Equal(Enum) (Variables|Default|GetCurrentState) "NewEnumerator2")
    (Variables|Default|SetCurrentState "NewEnumerator0")))

(event OnComponentHit(TargetBoard)
  (params (HitComponent :type Primitive%20Component%20Object%20Reference) (OtherActor :type Actor%20Object%20Reference) (OtherComp :type Primitive%20Component%20Object%20Reference) (NormalImpulse :type Vector :default "0, 0, 0") (Hit :type Hit%20Result%20Structure%20%28by%20ref%29))
  (Utilities|Casting|CastToBP_Bullet OtherActor)
  (CallFunction|KnockDown))

(event EventTick
  (params (DeltaSeconds :type Float%20%28single-precision%29))
  (CallFunction|TickRotate DeltaSeconds))

(fn ConstructionScript)

(fn StandUp
  (if (Utilities|Enum|Equal(Enum) (Variables|Default|GetCurrentState) "NewEnumerator0")
    (Utilities|FlowControl|Sequence
      (:then_0
        (bind _output_get (Variables|Rotation|SetRotationTime (Variables|Rotation|GetRotationTimeStandUp)))
        (Variables|Rotation|SetRotationRemainingTime _output_get))
      (:then_1
        (Variables|Rotation|SetRotationDegree -9e+01))
      (:then_2
        (Variables|Default|SetCurrentState "NewEnumerator4")))))

(fn KnockDown
  (if (Utilities|Enum|Equal(Enum) (Variables|Default|GetCurrentState) "NewEnumerator1")
    (Utilities|FlowControl|Sequence
      (:then_0
        (bind _output_get (Variables|Rotation|SetRotationTime (Variables|Rotation|GetRotationTimeKnockDown)))
        (Variables|Rotation|SetRotationRemainingTime _output_get))
      (:then_1
        (Variables|Rotation|SetRotationDegree 9e+01))
      (:then_2
        (Variables|Default|SetCurrentState "NewEnumerator3"))
      (:then_3
        (CallFunction|AddScore (Variables|Default|GetScoreWhenKnockDown))))))

(fn TickRotate
  (params (DeltaTime :type Float%20%28double-precision%29))
  (if (>= (Variables|Rotation|GetRotationRemainingTime) 0.0)
    (Transformation|AddActorLocalRotation (Math|Rotator|MakeRotator 0.0 (* DeltaTime (/ (Variables|Rotation|GetRotationDegree) (Variables|Rotation|GetRotationTime))) 0.0) false false)
    (bind _output_get (Variables|Rotation|SetRotationRemainingTime (- (Variables|Rotation|GetRotationRemainingTime) DeltaTime)))
    (if (< _output_get 0.0)
      (switch Utilities|FlowControl|Switch|SwitchonSpartaTargetState (Variables|Default|GetCurrentState)
        (:NewEnumerator4
          (Variables|Default|SetCurrentState "NewEnumerator1"))
        (:NewEnumerator3
          (Variables|Default|SetCurrentState "NewEnumerator2"))))))