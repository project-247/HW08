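; BP_Bullet is a projectile actor that flies in a straight line and destroys itself on impact, with no damage logic of its own.
; Each Tick it moves with a swept SetActorLocation along the Bullet component's forward vector, scaled by Speed and delta time, without a projectile movement component.
; BeginPlay shrinks the Bullet component, its hit event destroys the actor, and SetSpeed exposes a setter for Speed.
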(event OnComponentHit(Bullet)
  (params (HitComponent :type Primitive%20Component%20Object%20Reference) (OtherActor :type Actor%20Object%20Reference) (OtherComp :type Primitive%20Component%20Object%20Reference) (NormalImpulse :type Vector :default "0, 0, 0") (Hit :type Hit%20Result%20Structure%20%28by%20ref%29))
  (Actor|DestroyActor))

(event EventBeginPlay
  (Transformation|SetWorldScale3D (Variables|Default|GetBullet) "0.100000,0.100000,0.100000"))

(event Collision|EventActorBeginOverlap
  (params (OtherActor :type Actor%20Object%20Reference)))

(event EventTick
  (params (DeltaSeconds :type Float%20%28single-precision%29))
  (Transformation|SetActorLocation (+ (CallFunction|CalculateMoveVector DeltaSeconds) (Transformation|GetActorLocation)) true false))

(fn ConstructionScript)

(fn CalculateMoveVector
  (params (Delta :type Float%20%28double-precision%29))
  (bind _bullet (Variables|Default|GetBullet))
  (bind _returnvalue (Math|Vector|GetForwardVector _bullet))
  (bind (_x _y _z) (Math|Vector|BreakVector _returnvalue))
  (LocalVariables|SetDeltaSpeed (* Delta (Variables|Default|GetSpeed)))
  (return (Math|Vector|MakeVector (* _x (LocalVariables|GetDeltaSpeed)) (* _y (LocalVariables|GetDeltaSpeed)) (* _z (LocalVariables|GetDeltaSpeed)))))

(fn SetSpeed
  (params (Value :type Float%20%28double-precision%29))
  (Variables|Default|SetSpeed Value))