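; BP_Gun is a gun with limited ammo and switchable semi-auto and full-auto fire modes.
; Fire spends a bullet and spawns a BP_Bullet at FrontOfGun, and in full auto re-arms a timer that calls Fire again until release clears it or ammo runs out.
; Reload restores full ammo, and getters expose use type, name, fire mode, ammo and busy state.
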(event EventBeginPlay)

(event Collision|EventActorBeginOverlap
  (params (OtherActor :type Actor%20Object%20Reference)))

(event EventTick
  (params (DeltaSeconds :type Float%20%28single-precision%29)))

(fn ConstructionScript)

(fn Fire
  (if (> (Variables|Default|GetRemainingBullets) 0)
    (Math|Integer|DecrementInt (Variables|Default|GetRemainingBullets)
      (:%20%20
        (Utilities|FlowControl|Sequence
          (:then_1
            (bind _returnvalue (Game|SpawnActorfromClass "/Game/Gun/BP_Bullet.BP_Bullet_C" (Transformation|GetWorldTransform (Variables|Default|GetFrontOfGun)) "Undefined" "MultiplyWithRoot" 0 0))
            (Default|SetSpeed _returnvalue 1e+03))
          (:then_2
            (switch Utilities|FlowControl|Switch|SwitchonFireModeOfGun (Variables|Default|GetFireMode)
              (:NewEnumerator1
                (bind _returnvalue_2 (Utilities|Time|SetTimerbyFunctionName 0 "Fire" (Variables|Default|GetDurationPerFire)))
                (Variables|Default|SetTimerFire _returnvalue_2)))))))))

(fn Reload
  (Variables|Default|SetRemainingBullets (Variables|Default|GetMaxRemainingBullets)))

(fn GetUseType
  (return (Variables|Default|GetUseType)))

(fn ChangeFireMode
  (switch Utilities|FlowControl|Switch|SwitchonFireModeOfGun (Variables|Default|GetFireMode)
    (:NewEnumerator0
      (Variables|Default|SetFireMode "NewEnumerator1"))
    (:NewEnumerator1
      (Variables|Default|SetFireMode "NewEnumerator0"))))

(fn FirePressed
  (Variables|Default|SetIsFirePressed true)
  (CallFunction|Fire))

(fn FireReleased
  (Variables|Default|SetIsFirePressed false)
  (Utilities|Time|ClearandInvalidateTimerbyHandle (Variables|Default|GetTimerFire)))

(fn IsBusy
  (return (CallFunction|IsFiring)))

(fn IsFiring
  (return (and (Variables|Default|GetIsFirePressed) (Utilities|Time|IsTimerActivebyHandle (Variables|Default|GetTimerFire)))))

(fn GetWeaponName
  (return (Variables|Default|GetWeaponName)))

(fn GetFireMode
  (return (Variables|Default|GetFireMode)))

(fn GetRemainingBullets
  (return (Variables|Default|GetRemainingBullets)))

(fn GetMaxRemainingBullets
  (return (Variables|Default|GetMaxRemainingBullets)))