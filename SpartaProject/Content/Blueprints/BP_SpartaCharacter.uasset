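; BP_SpartaCharacter is a character Blueprint that carries two BP_Gun weapons, one in hand and one on the back.
; BeginPlay caches both guns from Child Actor components, and Enhanced Input actions forward fire, reload and fire-mode changes to the held gun.
; Main and Sub swap inputs check the held gun's use type before calling SwapGun, which reattaches the guns between components and exchanges references unless the held gun is busy.
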(event Input|EnhancedActionEvents|EnhancedInputActionIA_Fire
  (params (ActionValue :type Boolean) (ElapsedSeconds :type Float%20%28double-precision%29) (TriggeredSeconds :type Float%20%28double-precision%29) (InputAction :type Input%20Action%20Object%20Reference :default "/Game/Inputs/IA_Fire.IA_Fire"))
  (bind _guninhand (Variables|Default|GetGunInHand))
  (if ActionValue
    (Default|FirePressed _guninhand)
    (else
      (Default|FireReleased _guninhand))))

(event Input|EnhancedActionEvents|EnhancedInputActionIA_Reload
  (params (ActionValue :type Boolean) (ElapsedSeconds :type Float%20%28double-precision%29) (TriggeredSeconds :type Float%20%28double-precision%29) (InputAction :type Input%20Action%20Object%20Reference :default "/Game/Inputs/IA_Reload.IA_Reload"))
  (Default|Reload (Variables|Default|GetGunInHand)))

(event Input|EnhancedActionEvents|EnhancedInputActionIA_SwapMain
  (params (ActionValue :type Boolean) (ElapsedSeconds :type Float%20%28double-precision%29) (TriggeredSeconds :type Float%20%28double-precision%29) (InputAction :type Input%20Action%20Object%20Reference :default "/Game/Inputs/IA_SwapMain.IA_SwapMain"))
  (switch Utilities|FlowControl|Switch|SwitchonUseTypeOfGun (Default|GetUseType (Variables|Default|GetGunInHand))
    (:NewEnumerator1
      (CallFunction|SwapGun))))

(event Input|EnhancedActionEvents|EnhancedInputActionIA_SwapSub
  (params (ActionValue :type Boolean) (ElapsedSeconds :type Float%20%28double-precision%29) (TriggeredSeconds :type Float%20%28double-precision%29) (InputAction :type Input%20Action%20Object%20Reference :default "/Game/Inputs/IA_SwapSub.IA_SwapSub"))
  (switch Utilities|FlowControl|Switch|SwitchonUseTypeOfGun (Default|GetUseType (Variables|Default|GetGunInHand))
    (:NewEnumerator0
      (CallFunction|SwapGun))))

(event Input|EnhancedActionEvents|EnhancedInputActionIA_FireMode
  (params (ActionValue :type Boolean) (ElapsedSeconds :type Float%20%28double-precision%29) (TriggeredSeconds :type Float%20%28double-precision%29) (InputAction :type Input%20Action%20Object%20Reference :default "/Game/Inputs/IA_FireMode.IA_FireMode"))
  (Default|ChangeFireMode (Variables|Default|GetGunInHand)))

(event EventBeginPlay
  (bind _asbp_gun (Utilities|Casting|CastToBP_Gun (Variables|/Script/Engine.ChildActorComponent|GetChildActor (Variables|Default|GetWeaponInHand))))
  (Variables|Default|SetGunInHand _asbp_gun)
  (bind _asbp_gun_2 (Utilities|Casting|CastToBP_Gun (Variables|/Script/Engine.ChildActorComponent|GetChildActor (Variables|Default|GetWeaponInBack))))
  (Variables|Default|SetGunInBack _asbp_gun_2))

(fn ConstructionScript)

(fn SwapGun
  (if (not (Default|IsBusy (Variables|Default|GetGunInHand)))
    (LocalVariables|SetWillBeDrawn (Variables|Default|GetGunInBack))
    (LocalVariables|SetWillBePut (Variables|Default|GetGunInHand))
    (Transformation|AttachComponentToComponent (LocalVariables|GetWillBeDrawn) (Variables|Default|GetWeaponInHand) "None" "KeepRelative" "KeepRelative" "KeepRelative" true)
    (Transformation|AttachComponentToComponent (LocalVariables|GetWillBePut) (Variables|Default|GetWeaponInBack) "None" "KeepRelative" "KeepRelative" "KeepRelative" true)
    (Variables|Default|SetGunInHand (LocalVariables|GetWillBeDrawn))
    (Variables|Default|SetGunInBack (LocalVariables|GetWillBePut))))

(fn GetGuninHand
  (return (Variables|Default|GetGunInHand)))